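; BP_HealthPack is a health pickup that heals the player on overlap.
; When the HealthPack component begins overlapping an actor, it casts to BP_Player and passes it to AddHealth.
; AddHealth adds a fixed amount to the player's Health, capped at a hardcoded maximum, then destroys the pack.
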(event `self.HealthPack.OnComponentBeginOverlap`
  (params (OverlappedComponent :type "PrimitiveComponent Object Reference") (OtherActor :type "Actor Object Reference") (OtherComp :type "PrimitiveComponent Object Reference") (OtherBodyIndex :type Integer) (bFromSweep :type Boolean) (SweepResult :type "HitResult Structure (by ref)"))
  (bind _asbp_player (cast `/Game/InfiniteMatrix/Blueprints/BP_Player` OtherActor))
  (`self.AddHealth` _asbp_player)
  (`self.K2_DestroyActor`))

(fn `AddHealth`
  (params (`BP player` :type "/Game/InfiniteMatrix/Blueprints/BP_Player Object Reference"))
  (bind _returnvalue (+ (`/Game/InfiniteMatrix/Blueprints/BP_Player.Health` `BP player`) 20.0))
  (if (>= _returnvalue 100.0)
    (set `/Game/InfiniteMatrix/Blueprints/BP_Player.Health` 100.0 `BP player`)
    (else
      (set `/Game/InfiniteMatrix/Blueprints/BP_Player.Health` _returnvalue `BP player`)))
  (`self.K2_DestroyActor`))

(fn `UserConstructionScript`)