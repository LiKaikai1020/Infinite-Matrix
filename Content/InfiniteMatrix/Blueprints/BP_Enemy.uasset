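; BP_Enemy is an enemy actor that damages the player on contact and awards score when shot.
; Hitting BP_Player destroys the enemy, lowers the player's clamped Health, shows the restart display at zero and plays a camera shake.
; Overlapping a BP_Projectile destroys both actors and increments the player's Score.
; A separate TriggerZone destroys the enemy when the player overlaps it, without changing health or score.
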(event `self.Enemy.OnComponentHit`
  (params (HitComponent :type "PrimitiveComponent Object Reference") (OtherActor :type "Actor Object Reference") (OtherComp :type "PrimitiveComponent Object Reference") (NormalImpulse :type "Vector Structure") (Hit :type "HitResult Structure (by ref)"))
  (bind _asbp_player (cast `/Game/InfiniteMatrix/Blueprints/BP_Player` OtherActor))
  (`self.K2_DestroyActor`)
  (`self.UpdateHealth` _asbp_player)
  (`GameplayStatics.PlayWorldCameraShake` "/Game/InfiniteMatrix/Blueprints/BP_CSHAKE.BP_CSHAKE_C" (`self.K2_GetActorLocation` _asbp_player) 0.0 500.0))

(event `self.Enemy.OnComponentBeginOverlap`
  (params (OverlappedComponent :type "PrimitiveComponent Object Reference") (OtherActor :type "Actor Object Reference") (OtherComp :type "PrimitiveComponent Object Reference") (OtherBodyIndex :type Integer) (bFromSweep :type Boolean) (SweepResult :type "HitResult Structure (by ref)"))
  (bind _asbp_projectile (cast `/Game/InfiniteMatrix/Blueprints/BP_Projectile` OtherActor))
  (`self.K2_DestroyActor`)
  (`self.K2_DestroyActor` _asbp_projectile)
  (bind _returnvalue (`GameplayStatics.GetActorOfClass` "/Game/InfiniteMatrix/Blueprints/BP_Player.BP_Player_C"))
  (`self.UpdateScore` _returnvalue))

(event `self.TriggerZone.OnComponentBeginOverlap`
  (params (OverlappedComponent :type "PrimitiveComponent Object Reference") (OtherActor :type "Actor Object Reference") (OtherComp :type "PrimitiveComponent Object Reference") (OtherBodyIndex :type Integer) (bFromSweep :type Boolean) (SweepResult :type "HitResult Structure (by ref)"))
  (cast `/Game/InfiniteMatrix/Blueprints/BP_Player` OtherActor)
  (`self.K2_DestroyActor`))

(fn `UpdateHealth`
  (params (`BP Player` :type "/Game/InfiniteMatrix/Blueprints/BP_Player Object Reference"))
  (set `/Game/InfiniteMatrix/Blueprints/BP_Player.Health` (`KismetMathLibrary.FClamp` (- (`/Game/InfiniteMatrix/Blueprints/BP_Player.Health` `BP Player`) 20.0) 0.0 100.0) `BP Player`)
  (if (== (`/Game/InfiniteMatrix/Blueprints/BP_Player.Health` `BP Player`) 0.0)
    (`/Game/InfiniteMatrix/Blueprints/BP_Player.DisplayRestart` `BP Player`)))

(fn `UpdateScore`
  (params (`BP player` :type "/Game/InfiniteMatrix/Blueprints/BP_Player Object Reference"))
  (set `/Game/InfiniteMatrix/Blueprints/BP_Player.Score` (+ (`/Game/InfiniteMatrix/Blueprints/BP_Player.Score` `BP player`) 1) `BP player`)
  (`self.K2_DestroyActor`))

(fn `UserConstructionScript`)